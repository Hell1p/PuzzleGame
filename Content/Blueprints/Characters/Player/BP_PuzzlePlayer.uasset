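; First-person puzzle player character with camera head bob, crouching and automatic depth-of-field focus.
; Each tick picks an idle, walk or sprint camera shake from horizontal speed and jump ability.
; The crouch axis lowers walk speed and shrinks the capsule through a timeline, while an upward trace blocks standing under obstacles.
; A looping timer traces forward from the camera, setting focal distance to the hit and animating aperture through a timeline.
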(event Custom|HeadBob
  (bind _returnvalue (Game|GetPlayerController 0))
  (bind _charactermovement (Variables|Character|GetCharacterMovement))
  (bind _velocity (Variables|/Script/Engine.MovementComponent|GetVelocity _charactermovement))
  (bind _returnvalue_2 (Math|Vector|VectorLengthXY _velocity))
  ;[0.2923 0.4974 1] HeadBob Funcion
  (if (and (> _returnvalue_2 0.0) (Character|CanJump))
    (if (< _returnvalue_2 501.0)
      (Game|Feedback|ClientStartCameraShake _returnvalue "/Game/Blueprints/HeadBob/Walk.Walk_C" 1.0 "CameraLocal" "0, 0, 0")
      (else
        (Game|Feedback|ClientStartCameraShake _returnvalue "/Game/Blueprints/HeadBob/Sprint.Sprint_C" 1.0 "CameraLocal" "0, 0, 0")))
    (else
      (Game|Feedback|ClientStartCameraShake _returnvalue "/Game/Blueprints/HeadBob/Idle.Idle_C" 1.0 "CameraLocal" "0, 0, 0"))))

(event Custom|ADOF
  (bind _playercamera (Variables|Default|GetPlayerCamera))
  (bind _playercamera_2 (Variables|Default|GetPlayerCamera))
  (bind _returnvalue (Transformation|GetWorldLocation _playercamera))
  ;[0.5491 1 0.9502] Focusing
  (bind (_outhit _returnvalue_2) (Collision|LineTraceByChannel _returnvalue (+ _returnvalue (* (Math|Vector|GetForwardVector _playercamera) 1e+04)) "TraceTypeQuery1" false 0 "None"))
  (if _returnvalue_2
    (Variables|Default|SetFocusLocation (Math|Vector|VectorLength (- (.Location (Collision|BreakHitResult _outhit)) (Transformation|GetWorldLocation _playercamera_2))))
    (bind _newtrack_0 (Timeline|Depth Play)
      (:Update
        (Variables|/Script/Engine.CameraComponent|SetPostProcessSettings _playercamera_2 (Utilities|Struct|MakePostProcessSettings _newtrack_0 11.0 (Variables|Default|GetFocusLocation)))))))

(event Custom|CrouchTrace
  ;[1 1 1] TraceCrouch
  (bind _outhit (Collision|LineTraceByChannel (Transformation|GetWorldLocation (Variables|Default|GetPlayerCamera)) (+ (* (Math|Vector|GetUpVector (Variables|Default|GetCapsuleComponent)) 1e+02) (Transformation|GetWorldLocation (Variables|Default|GetPlayerCamera))) "TraceTypeQuery1" true 0 "ForDuration"))
  (Variables|Default|SetbBlockingHitR (.bBlockingHit (Collision|BreakHitResult _outhit))))

(event EventBeginPlay
  ;[0.2923 0.4974 1] HeadBob Funcion
  (Utilities|Time|SetTimerbyFunctionName 0 "ADOF" 0.2 true))

(event EventTick
  (params (DeltaSeconds :type Float%20%28single-precision%29))
  ;[0.2923 0.4974 1] HeadBob Funcion
  (CallFunction|HeadBob)
  (if (Variables|Default|GetbCrouching)
    (CallFunction|CrouchTrace)))

(event Input|AxisEvents|InputAxisAxisCrouch
  (params (AxisValue :type Float%20%28single-precision%29))
  (bind _charactermovement (Variables|Character|GetCharacterMovement))
  ;[1 0.5725 0.9072] CrouchFunction
  (if (> AxisValue 0.0)
    (Variables|/Script/Engine.CharacterMovementComponent|SetMaxWalkSpeed _charactermovement 3e+02)
    (Variables|Default|SetbCrouching true)
    (bind _newtrack_0 (Timeline|Timeline Play)
      (:Update
        (Components|Capsule|SetCapsuleHalfHeight (Variables|Default|GetCapsuleComponent) (Math|Float|Lerp 88.0 34.0 _newtrack_0) true)))
    (elif (not (Variables|Default|GetbBlockingHitR))
      (Variables|/Script/Engine.CharacterMovementComponent|SetMaxWalkSpeed _charactermovement 6e+02)
      (Variables|Default|SetbCrouching false)
      (Timeline|Timeline Reverse))))

(fn ConstructionScript)