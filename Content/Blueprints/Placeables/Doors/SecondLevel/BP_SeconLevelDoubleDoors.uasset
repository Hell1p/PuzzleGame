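; Second-level double door that swings open or closed when a BP_SecondLevelCard actor begins overlapping its Box trigger.
; Each qualifying overlap toggles two FlipFlops that play or reverse a separate Timeline for each leaf, setting the relative yaw of Door1 and Door2.
; There is no end-overlap handling, so the doors change state only when the card enters the box again.
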(event OnComponentBeginOverlap(Box)
  (params (OverlappedComponent :type Primitive%20Component%20Object%20Reference) (OtherActor :type Actor%20Object%20Reference) (OtherComp :type Primitive%20Component%20Object%20Reference) (OtherBodyIndex :type Integer) (bFromSweep :type Boolean) (SweepResult :type Hit%20Result%20Structure%20%28by%20ref%29))
  (bind _asbp_second_level_card (Utilities|Casting|CastToBP_SecondLevelCard OtherActor))
  (Utilities|IsValid _asbp_second_level_card
    (:Is%20Valid
      (Utilities|FlowControl|Sequence
        (:then_0
          (Utilities|FlowControl|FlipFlop
            (:A
              (bind _newtrack_0 (Timeline|Timeline Play)
                (:Update
                  (Transformation|SetRelativeRotation (Variables|Default|GetDoor2) (Math|Rotator|MakeRotator 0.0 0.0 _newtrack_0) false false))))
            (:B
              (Timeline|Timeline Reverse))))
        (:then_1
          (Utilities|FlowControl|FlipFlop
            (:A
              (bind _newtrack_0_2 (Timeline|Timeline_0 Play)
                (:Update
                  (Transformation|SetRelativeRotation (Variables|Default|GetDoor1) (Math|Rotator|MakeRotator 0.0 0.0 _newtrack_0_2) false false))))
            (:B
              (Timeline|Timeline_0 Reverse))))))))

(fn ConstructionScript)