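; A double door placeable that opens and closes when a first-level keycard enters its card reader's trigger box.
; Valid cards play a click and toggle two timelines forward or backward via FlipFlops, yawing each door leaf.
; One timeline also pulses an indicator light and sets a flag that ignores new swipes until it finishes.
; Other BP_BaseCard types trigger a failure sound and briefly flash a second light.
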(event OnComponentBeginOverlap(Box)
  (params (OverlappedComponent :type Primitive%20Component%20Object%20Reference) (OtherActor :type Actor%20Object%20Reference) (OtherComp :type Primitive%20Component%20Object%20Reference) (OtherBodyIndex :type Integer) (bFromSweep :type Boolean) (SweepResult :type Hit%20Result%20Structure%20%28by%20ref%29))
  (bind _asbp_base_card (Utilities|Casting|CastToBP_BaseCard OtherActor))
  (bind _asbp_first_level_card (Utilities|Casting|CastToBP_FirstLevelCard _asbp_base_card)
    (:then
      (Utilities|IsValid _asbp_first_level_card
        (:Is%20Valid
          (if (not (Variables|Default|GetbDoorIsOpeningNow))
            (Audio|PlaySoundatLocation "/Engine/VREditor/Sounds/UI/Click_on_Button_Cue.Click_on_Button_Cue" (Transformation|GetWorldLocation (Variables|Default|GetCardReader)) "0, 0, 0" 1.0 1.0 0.0 0 0 0 0)
            (Utilities|FlowControl|Sequence
              (:then_0
                (Utilities|FlowControl|FlipFlop
                  (:A
                    (bind _newtrack_0 (Timeline|Timeline Play)
                      (:Update
                        (Transformation|SetRelativeRotation (Variables|Default|GetDoor2) (Math|Rotator|MakeRotator 0.0 0.0 _newtrack_0) false false)
                        (Variables|Default|SetbDoorIsOpeningNow true)
                        (Rendering|Components|Light|SetIntensity (Variables|Default|GetPointLight) 1e+02)
                        (Utilities|FlowControl|Delay 0.1)
                        (Rendering|Components|Light|SetIntensity (Variables|Default|GetPointLight) 0.0))
                      (:Finished
                        (Variables|Default|SetbDoorIsOpeningNow false))))
                  (:B
                    (Timeline|Timeline Reverse))))
              (:then_1
                (Utilities|FlowControl|FlipFlop
                  (:A
                    (bind _newtrack_0_2 (Timeline|Timeline_0 Play)
                      (:Update
                        (Transformation|SetRelativeRotation (Variables|Default|GetDoor1) (Math|Rotator|MakeRotator 0.0 0.0 _newtrack_0_2) false false))))
                  (:B
                    (Timeline|Timeline_0 Reverse)))))))))
    (:CastFailed
      (Audio|PlaySoundatLocation "/Engine/EditorSounds/Notifications/CompileFailed_Cue.CompileFailed_Cue" (Transformation|GetWorldLocation (Variables|Default|GetCardReader)) "0, 0, 0" 0.3 1.0 0.0 0 0 0 0)
      (Rendering|Components|Light|SetIntensity (Variables|Default|GetPointLight1) 1e+02)
      (Utilities|FlowControl|Delay 0.2)
      (Rendering|Components|Light|SetIntensity (Variables|Default|GetPointLight1) 0.0))))

(fn ConstructionScript)